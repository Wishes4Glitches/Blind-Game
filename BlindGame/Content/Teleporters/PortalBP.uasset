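; PortalBP is a paired two-way teleporter that moves the FirstPersonCharacter between an entrance and an exit sharing a PortalIndex.
; On Hit it plays a 2D sound, then searches all PortalBP actors for the same index and opposite Entrance flag.
; The character takes the location and rotation of that portal's ExitReference.
; The Construction Script places the Portal and ExitReference components from transform variables.
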(event `self.ReceiveHit`
  (params (MyComp :type "PrimitiveComponent Object Reference") (Other :type "Actor Object Reference") (OtherComp :type "PrimitiveComponent Object Reference") (bSelfMoved :type Boolean) (HitLocation :type "Vector Structure") (HitNormal :type "Vector Structure") (NormalImpulse :type "Vector Structure") (Hit :type "HitResult Structure (by ref)"))
  (bind _asfirst_person_character (cast `/Game/FirstPersonBP/Blueprints/FirstPersonCharacter` Other))
  (`GameplayStatics.PlaySound2D` "/Engine/VREditor/Sounds/UI/Teleport_Committed.Teleport_Committed" 1.0 1.0 0.0 null null)
  (if (`self.Entrance?`)
    (bind _outactors (`GameplayStatics.GetAllActorsOfClass` "PortalBP_C"))
    (for _array_element _outactors
      (if (and (== (`/Game/Teleporters/PortalBP.Portal Index` _array_element) (`self.Portal Index`)) (not (`/Game/Teleporters/PortalBP.Entrance?` _array_element)))
        (break)))
    (bind _exit_reference (`/Game/Teleporters/PortalBP.Exit Reference` _array_element))
    (`self.K2_SetActorLocationAndRotation` _asfirst_person_character (`SceneComponent.K2_GetComponentLocation` _exit_reference) (`SceneComponent.K2_GetComponentRotation` _exit_reference) false false)
    (else
      (bind _outactors_2 (`GameplayStatics.GetAllActorsOfClass` "PortalBP_C"))
      (for _array_element_2 _outactors_2
        (if (and (== (`/Game/Teleporters/PortalBP.Portal Index` _array_element_2) (`self.Portal Index`)) (and (not (`self.Entrance?`)) (`/Game/Teleporters/PortalBP.Entrance?` _array_element_2)))
          (break)))
      (bind _exit_reference_2 (`/Game/Teleporters/PortalBP.Exit Reference` _array_element_2))
      (`self.K2_SetActorLocationAndRotation` _asfirst_person_character (`SceneComponent.K2_GetComponentLocation` _exit_reference_2) (`SceneComponent.K2_GetComponentRotation` _exit_reference_2) false false))))

(fn `UserConstructionScript`
  ;[1 1 1] set portal and exit location and rotation
  (`SceneComponent.K2_SetRelativeTransform` (`self.Portal`) (`self.Portal Transform`) false false)
  (`SceneComponent.K2_SetRelativeLocationAndRotation` (`self.Exit Reference`) (`self.Exit Location`) (`self.Exit Rotation`) false false))