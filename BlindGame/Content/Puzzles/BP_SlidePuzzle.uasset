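; Sliding tile puzzle actor that opens a linked BP_SlidePuzzleDoor when solved.
; The construction script builds a scaled grid of box slots and one fewer mesh tiles, each showing an offset slice of the texture, then optionally shuffles them randomly.
; A tile hit finds nearby slots by sphere overlap and slides the tile via timeline into the empty one.
; After each move, tile-to-slot overlaps determine whether it is solved.
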(event `self.ReceiveBeginPlay`)

(event `OnMeshHit`
  (params (HitComponent :type "PrimitiveComponent Object Reference") (OtherActor :type "Actor Object Reference") (OtherComp :type "PrimitiveComponent Object Reference") (NormalImpulse :type "Vector Structure") (Hit :type "HitResult Structure (by ref)"))
  ;[1 1 1] On event called, get the neighboring meshes, find an open space to move to, then move to it.
  (set `self.Clicked Mesh` HitComponent)
  (bind _neighbors (`self.GetNeighbors`))
  (`self.GetMoveTo` _neighbors)
  (`/Engine/EditorBlueprintResources/StandardMacros.IsValid` (`self.MoveToTarget`)
    (:`Is Valid`
      (if (`self.AllowMovement`)
        (`self.MoveTo`)))))

(event `MoveTo`
  (bind _clicked_mesh (`self.Clicked Mesh`))
  (bind _movetotarget (`self.MoveToTarget`))
  ;[1 1 1] Move Block to open space.
  (set `self.AllowMovement` false)
  (set `self.Move ToStart` (`SceneComponent.RelativeLocation` (`self.Clicked Mesh`)))
  (bind (_direction _newtrack_0) (`Timeline|Timeline_0` :!via `PlayFromStart`)
    (:`Update`
      (`/Engine/EditorBlueprintResources/StandardMacros.IsValid` _movetotarget
        (:`Is Valid`
          (`/Engine/EditorBlueprintResources/StandardMacros.IsValid` _clicked_mesh
            (:`Is Valid`
              (`SceneComponent.K2_SetRelativeLocation` _clicked_mesh (`KismetMathLibrary.VLerp` (`self.Move ToStart`) (`SceneComponent.RelativeLocation` _movetotarget) _newtrack_0) false false))))))
    (:`Finished`
      (set `self.AllowMovement` true)
      (bind _solved (`self.IsSolved?`))
      (if _solved
        (bind _asbp_slide_puzzle_door (cast `/Game/Puzzles/BP_SlidePuzzleDoor` (`self.Door`)))
        (`/Game/Puzzles/BP_SlidePuzzleDoor.OpenDoor` _asbp_slide_puzzle_door)))))

(fn `GetMoveTo`
  (params (`Neighbors List` :type "Array of PrimitiveComponent Object Reference"))
  (set `self.MoveToTarget` null)
  (for _array_element `Neighbors List`
    (if (not (`PrimitiveComponent.IsOverlappingActor` _array_element self))
      (set `self.MoveToTarget` _array_element)))
  (return))

(fn `GetNeighbors`
  (returns (Neighbors :type "Array of PrimitiveComponent Object Reference"))
  (bind _outcomponents (`KismetSystemLibrary.SphereOverlapComponents` (`SceneComponent.K2_GetComponentLocation` (`self.Clicked Mesh`)) (/ (`self.DesiredSize`) (`KismetMathLibrary.Conv_IntToDouble` (`self.GridSize`))) (`|MakeArray` "ObjectTypeQuery1" "ObjectTypeQuery2" :!type "EObjectTypeQuery Enum") "/Script/Engine.BoxComponent"))
  (return _outcomponents))

(fn `IsSolved?`
  (returns (Solved :type Boolean))
  (locals (Solve :type Boolean :default true))
  (for (_array_element _array_index) (`self.MeshesList`)
    (if (not (`PrimitiveComponent.IsOverlappingComponent` _array_element (`|GetArrayItem` (`self.SpacesList`) _array_index)))
      (set `local.Solve` false)
      (break)))
  (return (`local.Solve`)))

(fn `ScalePuzzle`
  (`self.SetActorScale3D` (/ (1.0 1.0 1.0) (/ (* (`self.GridSize`) (`self.MeshSize`)) (`self.DesiredSize`))))
  (return))

(fn `ShufflePuzzle`
  (locals (Locations :type "Array of Vector Structure"))
  (bind _locations (`local.Locations`))
  (if (`self.Shuffle?`)
    (for _array_element (`self.SpacesList`)
      (`KismetArrayLibrary.Array_Add` (`local.Locations`) (`SceneComponent.RelativeLocation` _array_element)))
    (`KismetArrayLibrary.Array_Shuffle` (`local.Locations`))
    (for _array_element_2 (`self.MeshesList`)
      (`SceneComponent.K2_SetRelativeLocation` _array_element_2 (`|GetArrayItem` _locations) false false)
      (`KismetArrayLibrary.Array_Remove` _locations))
    (return)
    (else
      (return))))

(fn `SpawnPuzzle`
  (bind _meshsize (`self.MeshSize`))
  (bind _spaceslist (`self.SpacesList`))
  (bind _mesheslist (`self.MeshesList`))
  (bind _meshsize_2 (`self.MeshSize`))
  (bind _returnvalue (- (`self.GridSize`) 1))
  (bind _returnvalue_2 (`KismetMathLibrary.Conv_IntToDouble` (`self.GridSize`)))
  (bind _returnvalue_3 (/ (`self.MeshSize`) 4.0))
  (bind _returnvalue_4 (- (`self.GridSize`) 1))
  (bind _returnvalue_5 (/ 1.0 _returnvalue_2))
  (bind (_arrayindex _arrayelement) (`/Engine/EditorBlueprintResources/StandardMacros.ReverseForEachLoop` _spaceslist)
    (:`LoopBody`
      (`ActorComponent.K2_DestroyComponent` _arrayelement))
    (:`Completed`
      (`KismetArrayLibrary.Array_Clear` _spaceslist)
      (bind (_arrayindex_2 _arrayelement_2) (`/Engine/EditorBlueprintResources/StandardMacros.ReverseForEachLoop` _mesheslist)
        (:`LoopBody`
          (`ActorComponent.K2_DestroyComponent` _arrayelement_2))
        (:`Completed`
          (`KismetArrayLibrary.Array_Clear` _mesheslist)
          (for _index (range (+ _returnvalue 1))
            (set `self.Y Index` _index)
            (for _index_2 (range (+ _returnvalue 1))
              (set `self.X Index` _index_2)
              (bind _returnvalue_6 (`AddComponent|NODE_AddBoxComponent-0` :`RelativeTransform` (`KismetMathLibrary.MakeTransform` (`KismetMathLibrary.MakeVector` (* (`self.X Index`) _meshsize) (* (`self.Y Index`) _meshsize)))))
              (`BoxComponent.SetBoxExtent` _returnvalue_6 (`KismetMathLibrary.MakeVector` _returnvalue_3 _returnvalue_3 _returnvalue_3) true)
              (`KismetArrayLibrary.Array_Add` (`self.SpacesList`) _returnvalue_6)
              (if (not (and (== (`self.X Index`) _returnvalue_4) (== (`self.Y Index`) _returnvalue_4)))
                (bind _returnvalue_7 (`AddComponent|NODE_AddStaticMeshComponent-0` :`RelativeTransform` (`KismetMathLibrary.MakeTransform` (`KismetMathLibrary.MakeVector` (* (`self.X Index`) _meshsize_2) (* (`self.Y Index`) _meshsize_2)))))
                (`KismetArrayLibrary.Array_Add` (`self.MeshesList`) _returnvalue_7)
                (bind _returnvalue_8 (`PrimitiveComponent.CreateDynamicMaterialInstance` _returnvalue_7 0 "/Game/Puzzles/M_SlidePuzzleMaterial.M_SlidePuzzleMaterial" "None"))
                (`MaterialInstanceDynamic.SetTextureParameterValue` _returnvalue_8 "SlidePuzzleTexture" (`self.Texture`))
                (`MeshComponent.SetVectorParameterValueOnMaterials` _returnvalue_7 "TextureOffset 2D" (`KismetMathLibrary.MakeVector` (* (`self.X Index`) _returnvalue_5) (* (`self.Y Index`) _returnvalue_5) _returnvalue_2)))))
          (return))))))

(fn `UserConstructionScript`
  (`self.SpawnPuzzle`)
  (`self.ShufflePuzzle`)
  (`self.ScalePuzzle`))